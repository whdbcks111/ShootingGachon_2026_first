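; BP_Player is the player actor, which moves on the Y-Z plane and fires bullets from two muzzle points.
; Horizontal and Vertical axis inputs share one setter for Direction, which Tick scales by Speed and DeltaSeconds for swept, frame-rate-independent movement.
; Pressing Fire calls FireBullet at FirePosition1 and FirePosition2, spawning a BP_Bullet at each, then plays a 2D blaster sound.
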(event EventBeginPlay)

(event EventTick
  (params (DeltaSeconds :type Float%20%28single-precision%29))
  ;[0.15 0.15 0.15 0.5] 이동한다.
  (Transformation|SetActorLocation (+ (* DeltaSeconds (* (Variables|Default|GetDirection) (Variables|Default|GetSpeed))) (Transformation|GetActorLocation)) true false))

(event Input|ActionEvents|InputActionFire
  (params (Key :type Key%20Structure :default "None"))
  (:Pressed
    (CallFunction|FireBullet (Transformation|GetWorldLocation (Variables|Default|GetFirePosition1)))
    (CallFunction|FireBullet (Transformation|GetWorldLocation (Variables|Default|GetFirePosition2)))
    (Audio|PlaySound2D "/Game/star-wars-blaster.star-wars-blaster" 1.0 1.0 0.0 0 0)))

(event Input|AxisEvents|InputAxisHorizontal
  (params (AxisValue :type Float%20%28single-precision%29))
  (Variables|Default|SetDirection (Math|Vector|MakeVector 0.0 AxisValue (stale Input|AxisEvents|InputAxisVertical AxisValue))))

(event Input|AxisEvents|InputAxisVertical
  (params (AxisValue :type Float%20%28single-precision%29))
  (Variables|Default|SetDirection (Math|Vector|MakeVector 0.0 (stale Input|AxisEvents|InputAxisHorizontal AxisValue) AxisValue)))

(fn ConstructionScript)

(fn FireBullet
  (params (Fire%20Position :type Vector))
  (Game|SpawnActorfromClass "/Game/Blueprints/BP_Bullet.BP_Bullet_C" (Math|Transform|MakeTransform Fire%20Position "0, 0, 0" "1.000000,1.000000,1.000000") "AlwaysSpawn" "MultiplyWithRoot" 0 0))