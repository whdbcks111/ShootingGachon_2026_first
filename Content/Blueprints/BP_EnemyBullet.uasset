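; BP_EnemyBullet is an enemy projectile that damages BP_Player on overlap, then destroys itself with an explosion effect and sound.
; On BeginPlay it aims once at the player, rotated around X by AngleOffset, or straight down without a target, and aligns its Z axis to that direction.
; Tick moves it in a straight line without sweeping, at a speed settable through SetSpeed.
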(event OnComponentBeginOverlap(Collision)
  (params (OverlappedComponent :type Primitive%20Component%20Object%20Reference) (OtherActor :type Actor%20Object%20Reference) (OtherComp :type Primitive%20Component%20Object%20Reference) (OtherBodyIndex :type Integer) (bFromSweep :type Boolean) (SweepResult :type Hit%20Result%20Structure%20%28by%20ref%29))
  ;[0.15 0.15 0.15 0.5] 플레이어랑 부딪히면 대미지를 준다
  (bind _asbp_player (Utilities|Casting|CastToBP_Player OtherActor))
  (Default|TakePlayerDamage _asbp_player 5.0)
  ;[0.15 0.15 0.15 0.5] 부딪히면 자신을 제거하고 폭발 효과를 낸다.
  (Actor|DestroyActor)
  (Niagara|SpawnSystematLocation "/Game/ExternalAssets/Fire_EXP_Vol01_Free/Niagara/EXP/NS_Sub_EXP_Mid_002_02.NS_Sub_EXP_Mid_002_02" (Transformation|GetActorLocation))
  (Audio|PlaySound2D "/Game/Sounds/Explosion.Explosion" 1.0 1.0 0.0 0 0))

(event EventBeginPlay
  ;[0.15 0.15 0.15 0.5] 타겟 초기화
  (bind _returnvalue (Actor|GetActorOfClass "/Game/Blueprints/BP_Player.BP_Player_C"))
  (Variables|Default|SetTarget _returnvalue)
  ;[0.15 0.15 0.15 0.5] 방향 지정
  (CallFunction|FindDirection)
  (Transformation|SetActorRotation (Math|Rotator|MakeRotfromZ (Variables|Default|GetDirection))))

(event EventTick
  (params (DeltaSeconds :type Float%20%28single-precision%29))
  ;[0.15 0.15 0.15 0.5] 이동 + 방향 조절
  (Transformation|SetActorLocation (+ (* DeltaSeconds (* (Variables|Default|GetDirection) (Variables|Default|GetSpeed))) (Transformation|GetActorLocation)) false false))

(fn ConstructionScript)

(fn FindDirection
  (Utilities|IsValid (Variables|Default|GetTarget)
    (:Is%20Valid
      (Variables|Default|SetDirection (Math|Vector|RotateVectorAroundAxis (Math|Vector|Normalize (- (Transformation|GetActorLocation (Variables|Default|GetTarget)) (Transformation|GetActorLocation))) (Variables|Default|GetAngleOffset) "1.000000,0.000000,0.000000")))
    (:Is%20Not%20Valid
      (Variables|Default|SetDirection "0.000000,0.000000,-1.000000"))))

(fn SetSpeed
  (params (New%20Speed :type Float%20%28double-precision%29))
  (Variables|Default|SetSpeed New%20Speed))